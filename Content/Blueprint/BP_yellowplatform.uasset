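; BP_yellowplatform is a moving platform Blueprint that stores its starting location at BeginPlay.
; A box trigger sets Canmove while BP_Player2 overlaps it and clears it when that player leaves.
; MoveForward, which nothing in this graph calls, checks that flag, then plays a timeline from the start.
; The timeline lerps the actor from its initial position to a fixed world Y offset, without sweeping.
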(event `self.ReceiveBeginPlay`
  (set `self.initialPos` (`self.K2_GetActorLocation`)))

(event `MoveForward`
  (if (`self.canmove`)
    (bind (_direction _newtrack_0) (`Timeline|Timeline` :!via `PlayFromStart`)
      (:`Update`
        (`self.K2_SetActorLocation` (`KismetMathLibrary.VLerp` (`self.initialPos`) (+ (`self.initialPos`) (0.0 320.0 0.0)) _newtrack_0))))))

(event `self.Box.OnComponentBeginOverlap`
  (params (OverlappedComponent :type "PrimitiveComponent Object Reference") (OtherActor :type "Actor Object Reference") (OtherComp :type "PrimitiveComponent Object Reference") (OtherBodyIndex :type Integer) (bFromSweep :type Boolean) (SweepResult :type "HitResult Structure (by ref)"))
  (cast `/Game/ThirdPerson/Blueprints/BP_Player2` OtherActor)
  (set `self.canmove` true))

(event `self.Box.OnComponentEndOverlap`
  (params (OverlappedComponent :type "PrimitiveComponent Object Reference") (OtherActor :type "Actor Object Reference") (OtherComp :type "PrimitiveComponent Object Reference") (OtherBodyIndex :type Integer))
  (cast `/Game/ThirdPerson/Blueprints/BP_Player2` OtherActor)
  (set `self.canmove` false))

(fn `UserConstructionScript`)