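; BP_Laserwall_2 is a laser wall that lowers and raises according to the state of the BP_wallButton_Big_Player2 button.
; Every Tick it looks up that button by class and reads IsLeave, calling RiseUp when true and RiseDown otherwise.
; Two timelines lerp the wall between its starting position and 250 units below.
; CanRiseup and CanRisedown flags block retriggering until the current move is nearly complete.
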(event `self.ReceiveBeginPlay`
  (set `self.canRisedown` true)
  (set `self.initialPosition` (`self.K2_GetActorLocation`)))

(event `RiseDown`
  (bind _returnvalue (`GameplayStatics.GetActorOfClass` "/Game/Blueprint/BP_wallButton_Big_Player2.BP_wallButton_Big_Player2_C"))
  (if (`/Game/Blueprint/BP_wallButton_Big_Player2.isLeave` _returnvalue)
    _
    (elif (`self.canRisedown`)
      (set `self.canRisedown` false)
      (set `self.canRiseup` false)
      (bind (_direction _newtrack_0) (`Timeline|Timeline` :!via `PlayFromStart`)
        (:`Update`
          (`self.K2_SetActorLocation` (`KismetMathLibrary.VLerp` (`self.initialPosition`) (- (`self.initialPosition`) (0.0 0.0 250.0)) _newtrack_0))
          (if (> _newtrack_0 0.95)
            (set `self.canRiseup` true)))))))

(event `RiseUp`
  (if (`self.canRiseup`)
    (set `self.canRiseup` false)
    (set `self.canRisedown` false)
    (bind (_direction _newtrack_0) (`Timeline|Timeline_0` :!via `PlayFromStart`)
      (:`Update`
        (`self.K2_SetActorLocation` (`KismetMathLibrary.VLerp` (- (`self.initialPosition`) (0.0 0.0 250.0)) (`self.initialPosition`) _newtrack_0))
        (if (> _newtrack_0 0.95)
          (set `self.canRisedown` true))))))

(event `self.ReceiveTick`
  (params (DeltaSeconds :type "Float (single-precision)"))
  (bind _returnvalue (`GameplayStatics.GetActorOfClass` "/Game/Blueprint/BP_wallButton_Big_Player2.BP_wallButton_Big_Player2_C"))
  (if (`/Game/Blueprint/BP_wallButton_Big_Player2.isLeave` _returnvalue)
    (`self.RiseUp`)
    (else
      (`self.RiseDown`))))

(fn `UserConstructionScript`)