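; BP_laser is a moving laser hazard that sweeps back and forth along world Y from its placed position.
; On BeginPlay a Timeline lerps the actor to a fixed offset, with IsReversed choosing the side, and alternates between forward and reverse playback to loop endlessly.
; Overlapping its Box calls PlayerRecover on BP_Player1.
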(event `self.ReceiveBeginPlay`
  (if (`self.isReversed`)
    (set `self.offsetPos` (0.0 -1300.0 0.0))
    (else
      (set `self.offsetPos` (0.0 1300.0 0.0))))
  (set `self.initialPos` (`self.K2_GetActorLocation`))
  (set `self.isForward` true)
  (bind (_direction _newtrack_0) (`Timeline|Timeline` :!label _label)
    (:`Update`
      (`self.K2_SetActorLocation` (`KismetMathLibrary.VLerp` (`self.initialPos`) (+ (`self.initialPos`) (`self.offsetPos`)) _newtrack_0)))
    (:`Finished`
      (if (`self.isForward`)
        (set `self.isForward` false)
        (goto _label :!via `Reverse`)
        (else
          (set `self.isForward` true)
          (goto _label :!via `PlayFromStart`))))))

(event `self.Box.OnComponentBeginOverlap`
  (params (OverlappedComponent :type "PrimitiveComponent Object Reference") (OtherActor :type "Actor Object Reference") (OtherComp :type "PrimitiveComponent Object Reference") (OtherBodyIndex :type Integer) (bFromSweep :type Boolean) (SweepResult :type "HitResult Structure (by ref)"))
  (bind _asbp_player_1 (cast `/Game/ThirdPerson/Blueprints/BP_Player1` OtherActor))
  (`/Game/ThirdPerson/Blueprints/BP_Player1.PlayerRecover` _asbp_player_1))

(fn `UserConstructionScript`)