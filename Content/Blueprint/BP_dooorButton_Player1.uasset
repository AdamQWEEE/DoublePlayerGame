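; BP_dooorButton_Player1 is a pressure button that responds only to BP_Player1 and helps drive a gate.
; Box overlap begin and end swap the Cylinder's material between glowing and plain red.
; The same events raise or lower ButtonOnNum on the BP_gate found with GetActorOfClass, so the button reports to a single gate through a shared count of pressed buttons.
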(event `self.Box.OnComponentBeginOverlap`
  (params (OverlappedComponent :type "PrimitiveComponent Object Reference") (OtherActor :type "Actor Object Reference") (OtherComp :type "PrimitiveComponent Object Reference") (OtherBodyIndex :type Integer) (bFromSweep :type Boolean) (SweepResult :type "HitResult Structure (by ref)"))
  (cast `/Game/ThirdPerson/Blueprints/BP_Player1` OtherActor)
  (`PrimitiveComponent.SetMaterial` (`self.Cylinder`) 0 "/Game/Material/M_buttonRedGlow.M_buttonRedGlow")
  (bind _returnvalue (`GameplayStatics.GetActorOfClass` "/Game/Blueprint/BP_gate.BP_gate_C"))
  (`/Engine/EditorBlueprintResources/StandardMacros.IsValid` _returnvalue
    (:`Is Valid`
      (set `/Game/Blueprint/BP_gate.buttonOnNum` (+ (`/Game/Blueprint/BP_gate.buttonOnNum` _returnvalue) 1) _returnvalue))))

(event `self.Box.OnComponentEndOverlap`
  (params (OverlappedComponent :type "PrimitiveComponent Object Reference") (OtherActor :type "Actor Object Reference") (OtherComp :type "PrimitiveComponent Object Reference") (OtherBodyIndex :type Integer))
  (cast `/Game/ThirdPerson/Blueprints/BP_Player1` OtherActor)
  (`PrimitiveComponent.SetMaterial` (`self.Cylinder`) 0 "/Game/Material/M_buttonRed.M_buttonRed")
  (bind _returnvalue (`GameplayStatics.GetActorOfClass` "/Game/Blueprint/BP_gate.BP_gate_C"))
  (`/Engine/EditorBlueprintResources/StandardMacros.IsValid` _returnvalue
    (:`Is Valid`
      (set `/Game/Blueprint/BP_gate.buttonOnNum` (- (`/Game/Blueprint/BP_gate.buttonOnNum` _returnvalue) 1) _returnvalue))))

(fn `UserConstructionScript`)