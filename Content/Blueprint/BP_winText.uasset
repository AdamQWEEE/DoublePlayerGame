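; BP_winText is a win-message actor that reveals its text render once its arrival count reaches two.
; It hides the text on BeginPlay, and the Box overlap increments PlayerArriveNum whenever BP_Player1 or BP_Player2 enters.
; Tick polls for a count of exactly two to show the text.
; The count never decrements or tracks which player entered, so one player re-entering also counts.
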(event `self.ReceiveBeginPlay`
  (`SceneComponent.SetVisibility` (`self.TextRender`) false false))

(event `self.ReceiveTick`
  (params (DeltaSeconds :type "Float (single-precision)"))
  (if (== (`self.playerArriveNum`) 2)
    (`SceneComponent.SetVisibility` (`self.TextRender`) true false)))

(event `self.Box.OnComponentBeginOverlap`
  (params (OverlappedComponent :type "PrimitiveComponent Object Reference") (OtherActor :type "Actor Object Reference") (OtherComp :type "PrimitiveComponent Object Reference") (OtherBodyIndex :type Integer) (bFromSweep :type Boolean) (SweepResult :type "HitResult Structure (by ref)"))
  (`|ExecutionSequence`
    (:`then_0`
      (cast `/Game/ThirdPerson/Blueprints/BP_Player1` OtherActor))
    (:`then_1`
      (cast `/Game/ThirdPerson/Blueprints/BP_Player2` OtherActor)))
  (set `self.playerArriveNum` (+ (`self.playerArriveNum`) 1)))

(fn `UserConstructionScript`)