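; BP_wallButton_small_Player2 is an overlap button that only a small Player 2 can trigger to operate a laser wall.
; When BP_Player2 enters the Box with IsSmall set, it calls RiseDown on the BP_Laserwall_1 found by class lookup and switches the Cylinder to a glowing red material.
; Any BP_Player2 exit restores the plain red material and sets IsLeave, without calling the wall.
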(event `self.Box.OnComponentBeginOverlap`
  (params (OverlappedComponent :type "PrimitiveComponent Object Reference") (OtherActor :type "Actor Object Reference") (OtherComp :type "PrimitiveComponent Object Reference") (OtherBodyIndex :type Integer) (bFromSweep :type Boolean) (SweepResult :type "HitResult Structure (by ref)"))
  (bind _asbp_player_2 (cast `/Game/ThirdPerson/Blueprints/BP_Player2` OtherActor))
  (if (`/Game/ThirdPerson/Blueprints/BP_Player2.isSmall` _asbp_player_2)
    (bind _returnvalue (`GameplayStatics.GetActorOfClass` "/Game/Blueprint/BP_Laserwall_1.BP_Laserwall_1_C"))
    (`/Game/Blueprint/BP_Laserwall_1.RiseDown` _returnvalue)
    (`PrimitiveComponent.SetMaterial` (`self.Cylinder`) 0 "/Game/Material/M_buttonRedGlow.M_buttonRedGlow")
    (set `self.isLeave` false)))

(event `self.Box.OnComponentEndOverlap`
  (params (OverlappedComponent :type "PrimitiveComponent Object Reference") (OtherActor :type "Actor Object Reference") (OtherComp :type "PrimitiveComponent Object Reference") (OtherBodyIndex :type Integer))
  (cast `/Game/ThirdPerson/Blueprints/BP_Player2` OtherActor)
  (set `self.isLeave` true)
  (`PrimitiveComponent.SetMaterial` (`self.Cylinder`) 0 "/Game/Material/M_buttonRed.M_buttonRed"))

(fn `UserConstructionScript`)