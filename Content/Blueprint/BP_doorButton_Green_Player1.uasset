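; Green floor or door button that only responds to BP_Player1, lowering an obstacle when that player enters its Box trigger.
; Begin overlap calls RiseDown on the BP_Obstacle found by GetActorOfClass, applies a green glow material to the Cylinder and clears IsLeave.
; End overlap sets IsLeave and restores the default material.
; The RiseUp call is disconnected, so this Blueprint never raises the obstacle again.
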(event `self.Box.OnComponentBeginOverlap`
  (params (OverlappedComponent :type "PrimitiveComponent Object Reference") (OtherActor :type "Actor Object Reference") (OtherComp :type "PrimitiveComponent Object Reference") (OtherBodyIndex :type Integer) (bFromSweep :type Boolean) (SweepResult :type "HitResult Structure (by ref)"))
  (cast `/Game/ThirdPerson/Blueprints/BP_Player1` OtherActor)
  (bind _returnvalue (`GameplayStatics.GetActorOfClass` "/Game/Blueprint/BP_Obstacle.BP_Obstacle_C"))
  (`/Game/Blueprint/BP_Obstacle.RiseDown` _returnvalue)
  (`PrimitiveComponent.SetMaterial` (`self.Cylinder`) 0 "/Game/ThirdPerson/M_greenglow.M_greenglow")
  (set `self.isLeave` false))

(event `self.Box.OnComponentEndOverlap`
  (params (OverlappedComponent :type "PrimitiveComponent Object Reference") (OtherActor :type "Actor Object Reference") (OtherComp :type "PrimitiveComponent Object Reference") (OtherBodyIndex :type Integer))
  (cast `/Game/ThirdPerson/Blueprints/BP_Player1` OtherActor)
  (set `self.isLeave` true)
  (`PrimitiveComponent.SetMaterial` (`self.Cylinder`) 0 "/Game/ThirdPerson/MI_ThirdPersonColWay.MI_ThirdPersonColWay"))

(fn `UserConstructionScript`)