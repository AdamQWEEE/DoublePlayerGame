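; BP_Colorplatform_red is a red platform that briefly vanishes after BP_Player1 steps on it, unless it has been made solid.
; Box overlap opens a window for changing it, then after a short delay a non-solid Plane loses collision and visibility before both return.
; ChangeSolid, not called within this Blueprint, works only during that window, setting IsSolid and the solid red material, with no revert.
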(event `self.Box.OnComponentBeginOverlap`
  (params (OverlappedComponent :type "PrimitiveComponent Object Reference") (OtherActor :type "Actor Object Reference") (OtherComp :type "PrimitiveComponent Object Reference") (OtherBodyIndex :type Integer) (bFromSweep :type Boolean) (SweepResult :type "HitResult Structure (by ref)"))
  (bind _plane (`self.Plane`))
  (bind _plane_2 (`self.Plane`))
  (cast `/Game/ThirdPerson/Blueprints/BP_Player1` OtherActor)
  (set `self.canchangeSolid` true)
  (`KismetSystemLibrary.Delay` 0.6)
  (if (not (`self.isSolid`))
    (set `self.canchangeSolid` false)
    (`PrimitiveComponent.SetCollisionEnabled` _plane_2 "NoCollision")
    (`SceneComponent.SetVisibility` _plane_2 false false)
    (`KismetSystemLibrary.Delay` 0.6)
    (`PrimitiveComponent.SetCollisionEnabled` _plane "QueryAndPhysics")
    (`SceneComponent.SetVisibility` _plane true false)))

(event `self.Box.OnComponentEndOverlap`
  (params (OverlappedComponent :type "PrimitiveComponent Object Reference") (OtherActor :type "Actor Object Reference") (OtherComp :type "PrimitiveComponent Object Reference") (OtherBodyIndex :type Integer))
  (cast `/Game/ThirdPerson/Blueprints/BP_Player1` OtherActor)
  (set `self.canchangeSolid` false))

(event `ChangeSolid`
  (if (`self.canchangeSolid`)
    (`KismetSystemLibrary.PrintString` "玩家站在上面了")
    (set `self.isSolid` true)
    (`PrimitiveComponent.SetMaterial` (`self.Plane`) 0 "/Game/ThirdPerson/M_redcube_solid.M_redcube_solid")))

(fn `UserConstructionScript`)