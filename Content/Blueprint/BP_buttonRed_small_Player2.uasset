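; Red floor button actor that responds only to Player 2, and only lights up while that player is small.
; Box overlap begin casts to BP_Player2, checks IsSmall, then sets the player's InteractText and swaps the Cylinder to a glowing red material.
; Overlap end clears the text and restores the plain material for Player 2 regardless of size.
; It only changes visuals and text, triggering nothing else.
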(event `self.Box.OnComponentBeginOverlap`
  (params (OverlappedComponent :type "PrimitiveComponent Object Reference") (OtherActor :type "Actor Object Reference") (OtherComp :type "PrimitiveComponent Object Reference") (OtherBodyIndex :type Integer) (bFromSweep :type Boolean) (SweepResult :type "HitResult Structure (by ref)"))
  (bind _asbp_player_2 (cast `/Game/ThirdPerson/Blueprints/BP_Player2` OtherActor))
  (if (`/Game/ThirdPerson/Blueprints/BP_Player2.isSmall` _asbp_player_2)
    (set `/Game/ThirdPerson/Blueprints/BP_Player2.interactText` "Button is On" _asbp_player_2)
    (`PrimitiveComponent.SetMaterial` (`self.Cylinder`) 0 "/Game/Material/M_buttonRedGlow.M_buttonRedGlow")))

(event `self.Box.OnComponentEndOverlap`
  (params (OverlappedComponent :type "PrimitiveComponent Object Reference") (OtherActor :type "Actor Object Reference") (OtherComp :type "PrimitiveComponent Object Reference") (OtherBodyIndex :type Integer))
  (bind _asbp_player_2 (cast `/Game/ThirdPerson/Blueprints/BP_Player2` OtherActor))
  (set `/Game/ThirdPerson/Blueprints/BP_Player2.interactText` "" _asbp_player_2)
  (`PrimitiveComponent.SetMaterial` (`self.Cylinder`) 0 "/Game/Material/M_buttonRed.M_buttonRed"))

(fn `UserConstructionScript`)