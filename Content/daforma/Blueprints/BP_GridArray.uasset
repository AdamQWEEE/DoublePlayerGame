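; BP_GridArray fills an X by Y grid, spaced by SectorSize, with instances of a chosen mesh on a HierarchicalInstancedStaticMesh.
; The construction script calls the Grid event, which uses a 2D grid macro to add one uniformly scaled instance per cell center.
; Roll and pitch scale with each cell's row indices for progressive rotation.
; Mesh and two material overrides are reapplied per cell, materials only where the slot already holds one.
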(event `Grid`
  (bind _hierarchicalinstancedstaticmesh (`self.HierarchicalInstancedStaticMesh`))
  (bind _instance_transform_scale (`self.Instance Transform Scale`))
  (bind (_current_point _total_points _0_1_phase _poly_center _x_row _y_row) (`/Engine/ArtTools/RenderToTexture/Macros/RenderToTextureMacros.2D Grid Execution Macro` (`self.Sector Size`) (0.0 0.0 0.0) (`self.X`) (`self.Y`))
    (:`Per Poly Execution`
      (`StaticMeshComponent.SetStaticMesh` _hierarchicalinstancedstaticmesh (`self.New Mesh`))
      (`InstancedStaticMeshComponent.AddInstance` _hierarchicalinstancedstaticmesh (`KismetMathLibrary.MakeTransform` _poly_center (`KismetMathLibrary.MakeRotator` (`KismetMathLibrary.Conv_IntToDouble` (* _x_row (`self.RotateX`))) (`KismetMathLibrary.Conv_IntToDouble` (* _y_row (`self.RotateY`)))) (`KismetMathLibrary.MakeVector` _instance_transform_scale _instance_transform_scale _instance_transform_scale)) false)
      (if (`KismetSystemLibrary.IsValid` (`PrimitiveComponent.GetMaterial` _hierarchicalinstancedstaticmesh 0))
        (`PrimitiveComponent.SetMaterial` _hierarchicalinstancedstaticmesh 0 (`self.Material_0`)))
      (if (`KismetSystemLibrary.IsValid` (`PrimitiveComponent.GetMaterial` _hierarchicalinstancedstaticmesh 1))
        (`PrimitiveComponent.SetMaterial` _hierarchicalinstancedstaticmesh 1 (`self.Material_1`))))))

(fn `UserConstructionScript`
  (`self.Grid`))