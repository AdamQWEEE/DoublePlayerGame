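; BP_Transform is an effector actor that drives a material transform effect, apparently world position offset, through the MPC_WPO parameter collection.
; Start writes its location, radius and rotation, scale, randomization and emissive settings to the collection, matches the Sphere to the radius, and overrides hardness at small radii.
; The construction script runs Start and calls Setparameter on BP_Controller, while BeginPlay repeats Start on a looping timer rather than Tick.
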(event `Initialize`
  (bind _returnvalue (`GameplayStatics.GetActorOfClass` "/Game/daforma/Blueprints/BP_Controller.BP_Controller_C"))
  (`/Game/daforma/Blueprints/BP_Controller.setparameter` _returnvalue))

(event `self.ReceiveBeginPlay`
  (`KismetSystemLibrary.K2_SetTimerDelegate` (delegate `Start`) 0.35 true))

(event `Start`
  (bind _radius (`self.Radius`))
  (`|ExecutionSequence`
    (:`then_0`
      (`KismetMaterialLibrary.SetScalarParameterValue` "/Game/daforma/Materials/MPC_WPO.MPC_WPO" "TransformRadius" (`self.Radius`))
      (bind _returnvalue (`KismetMaterialLibrary.GetScalarParameterValue` "/Game/daforma/Materials/MPC_WPO.MPC_WPO" "TransformRadius"))
      (bind _output_get (set `self.Radius` _returnvalue))
      (`SphereComponent.SetSphereRadius` (`self.Sphere`) _output_get true)
      (`KismetMaterialLibrary.SetVectorParameterValue` "/Game/daforma/Materials/MPC_WPO.MPC_WPO" "TransformPosition" (`KismetMathLibrary.Conv_VectorToLinearColor` (`self.K2_GetActorLocation`)))
      (if (<= _radius 0.0)
        (set `self.Hardness` -100.0)
        (elif (<= _radius 1.0)
          (set `self.Hardness` 0.0)
          (else
            (set `self.Hardness` (`self.Hardness`))))))
    (:`then_1`
      (`KismetMaterialLibrary.SetScalarParameterValue` "/Game/daforma/Materials/MPC_WPO.MPC_WPO" "TransformHardness" (`self.Hardness`))
      (`KismetMaterialLibrary.SetScalarParameterValue` "/Game/daforma/Materials/MPC_WPO.MPC_WPO" "TransformRotateIntensity" (`self.RotateIntensity`))
      (`KismetMaterialLibrary.SetVectorParameterValue` "/Game/daforma/Materials/MPC_WPO.MPC_WPO" "TransformDirection" (`self.RotateAxis`))
      (`KismetMaterialLibrary.SetScalarParameterValue` "/Game/daforma/Materials/MPC_WPO.MPC_WPO" "TransformTime" (`self.TransformTime`))
      (`KismetMaterialLibrary.SetScalarParameterValue` "/Game/daforma/Materials/MPC_WPO.MPC_WPO" "AffectRadius" (`KismetMathLibrary.Conv_BoolToDouble` (`self.RadiusMask`)))
      (`KismetMaterialLibrary.SetScalarParameterValue` "/Game/daforma/Materials/MPC_WPO.MPC_WPO" "RandomEmissive" (`KismetMathLibrary.Conv_BoolToDouble` (`self.RandomEmissive`)))
      (`KismetMaterialLibrary.SetScalarParameterValue` "/Game/daforma/Materials/MPC_WPO.MPC_WPO" "RandomEmissiveTime" (`self.RandomEmissiveTime`))
      (`KismetMaterialLibrary.SetScalarParameterValue` "/Game/daforma/Materials/MPC_WPO.MPC_WPO" "RandomSeed" (`self.RandomSeed`))
      (`KismetMaterialLibrary.SetScalarParameterValue` "/Game/daforma/Materials/MPC_WPO.MPC_WPO" "ModifierEmissive" (`KismetMathLibrary.Conv_BoolToDouble` (`self.ModifierEmissive`)))
      (`KismetMaterialLibrary.SetScalarParameterValue` "/Game/daforma/Materials/MPC_WPO.MPC_WPO" "TransformRotationOffset" (`self.RotationOffset`))
      (`KismetMaterialLibrary.SetScalarParameterValue` "/Game/daforma/Materials/MPC_WPO.MPC_WPO" "TransformIdleRotateAnimation" (`KismetMathLibrary.Conv_BoolToDouble` (`self.IdleRotateAnimation`)))
      (`KismetMaterialLibrary.SetScalarParameterValue` "/Game/daforma/Materials/MPC_WPO.MPC_WPO" "TransformIdleScaleAnimation" (`KismetMathLibrary.Conv_BoolToDouble` (`self.IdleScaleAnimation`)))
      (`KismetMaterialLibrary.SetScalarParameterValue` "/Game/daforma/Materials/MPC_WPO.MPC_WPO" "TransforEmissiveTweakPower" (`self.ModifierEmissiveTweak`))
      (`KismetMaterialLibrary.SetVectorParameterValue` "/Game/daforma/Materials/MPC_WPO.MPC_WPO" "TransformScale" (`self.TransformScaleAxis`))
      (`KismetMaterialLibrary.SetScalarParameterValue` "/Game/daforma/Materials/MPC_WPO.MPC_WPO" "TransformRandomizeRotation" (`KismetMathLibrary.Conv_BoolToDouble` (`self.RandomizeRotation`)))
      (`KismetMaterialLibrary.SetScalarParameterValue` "/Game/daforma/Materials/MPC_WPO.MPC_WPO" "TransformRandomizeScale" (`KismetMathLibrary.Conv_BoolToDouble` (`self.RandomizeScale`)))
      (`KismetMaterialLibrary.SetScalarParameterValue` "/Game/daforma/Materials/MPC_WPO.MPC_WPO" "TransformScaleIntesity" (`self.ScaleIntesity`))
      (`KismetMaterialLibrary.SetScalarParameterValue` "/Game/daforma/Materials/MPC_WPO.MPC_WPO" "TransformScaleOffset" (`self.ScaleOffset`))
      (`KismetMaterialLibrary.SetScalarParameterValue` "/Game/daforma/Materials/MPC_WPO.MPC_WPO" "TransformRandomizeScaleTweak" (`self.RandomizeScaleTweak`))
      (`KismetMaterialLibrary.SetScalarParameterValue` "/Game/daforma/Materials/MPC_WPO.MPC_WPO" "DefaultEmissiveIntesity" (`self.Default Emissive Intesity`))
      (`KismetMaterialLibrary.SetScalarParameterValue` "/Game/daforma/Materials/MPC_WPO.MPC_WPO" "RandomEmissiveIntesity" (`self.RandomEmissiveIntesity`)))))

(fn `UserConstructionScript`
  (`self.Start`)
  (`self.Initialize`))