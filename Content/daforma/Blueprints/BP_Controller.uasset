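; BP_Controller is a central controller that pushes shared emissive, radius mask and random seed settings to the Wave, Jitter, Rotate, Transform and Ripple effect actors.
; Setparameter finds one actor of each class, copies the variables onto it and calls its Start.
; It runs from the construction script and on a looping 0.35-second timer from BeginPlay.
; Ripple differs: its RandomEmissiveIntesity receives RandomEmissiveTime.
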(event `self.ReceiveBeginPlay`
  (`KismetSystemLibrary.K2_SetTimerDelegate` (delegate `setparameter`) 0.35 true))

(event `setparameter`
  (bind _radiusmask (`self.RadiusMask`))
  (bind _randomemissive (`self.RandomEmissive`))
  (bind _modifieremissive (`self.ModifierEmissive`))
  (bind _default_emissive_intesity (`self.Default Emissive Intesity`))
  (bind _randomemissivetime (`self.RandomEmissiveTime`))
  (bind _randomseed (`self.RandomSeed`))
  (bind _random_emissive_intesity (`self.Random Emissive Intesity`))
  (`|ExecutionSequence`
    (:`then_0`
      (bind _returnvalue (`GameplayStatics.GetActorOfClass` "/Game/daforma/Blueprints/BP_Wave.BP_Wave_C"))
      (set `/Game/daforma/Blueprints/BP_Wave.RandomEmissiveIntesity` _random_emissive_intesity _returnvalue)
      (set `/Game/daforma/Blueprints/BP_Wave.RadiusMask` _radiusmask _returnvalue)
      (set `/Game/daforma/Blueprints/BP_Wave.RandomEmissive` _randomemissive _returnvalue)
      (set `/Game/daforma/Blueprints/BP_Wave.ModifierEmissive` _modifieremissive _returnvalue)
      (set `/Game/daforma/Blueprints/BP_Wave.RandomSeed` _randomseed _returnvalue)
      (set `/Game/daforma/Blueprints/BP_Wave.RandomEmissiveTime` _randomemissivetime _returnvalue)
      (set `/Game/daforma/Blueprints/BP_Wave.DefaultEmissiveIntesity` _default_emissive_intesity _returnvalue)
      (`/Game/daforma/Blueprints/BP_Wave.Start` _returnvalue))
    (:`then_1`
      (bind _returnvalue_2 (`GameplayStatics.GetActorOfClass` "/Game/daforma/Blueprints/BP_Jitter.BP_Jitter_C"))
      (set `/Game/daforma/Blueprints/BP_Jitter.Random Emissive Intesity` _random_emissive_intesity _returnvalue_2)
      (set `/Game/daforma/Blueprints/BP_Jitter.RadiusMask` _radiusmask _returnvalue_2)
      (set `/Game/daforma/Blueprints/BP_Jitter.RandomEmissive` _randomemissive _returnvalue_2)
      (set `/Game/daforma/Blueprints/BP_Jitter.ModifierEmissive` _modifieremissive _returnvalue_2)
      (set `/Game/daforma/Blueprints/BP_Jitter.RandomSeed` _randomseed _returnvalue_2)
      (set `/Game/daforma/Blueprints/BP_Jitter.RandomEmissiveTime` _randomemissivetime _returnvalue_2)
      (set `/Game/daforma/Blueprints/BP_Jitter.DefaultEmissiveIntesity` _default_emissive_intesity _returnvalue_2)
      (`/Game/daforma/Blueprints/BP_Jitter.Start` _returnvalue_2))
    (:`then_2`
      (bind _returnvalue_3 (`GameplayStatics.GetActorOfClass` "/Game/daforma/Blueprints/BP_Rotate.BP_Rotate_C"))
      (set `/Game/daforma/Blueprints/BP_Rotate.RandomEmissiveIntesity` _random_emissive_intesity _returnvalue_3)
      (set `/Game/daforma/Blueprints/BP_Rotate.RadiusMask` _radiusmask _returnvalue_3)
      (set `/Game/daforma/Blueprints/BP_Rotate.RandomEmissive` _randomemissive _returnvalue_3)
      (set `/Game/daforma/Blueprints/BP_Rotate.ModifierEmissive` _modifieremissive _returnvalue_3)
      (set `/Game/daforma/Blueprints/BP_Rotate.RandomSeed` _randomseed _returnvalue_3)
      (set `/Game/daforma/Blueprints/BP_Rotate.RandomEmissiveTime` _randomemissivetime _returnvalue_3)
      (set `/Game/daforma/Blueprints/BP_Rotate.DefaultEmissiveIntesity` _default_emissive_intesity _returnvalue_3)
      (`/Game/daforma/Blueprints/BP_Rotate.Start` _returnvalue_3))
    (:`then_3`
      (bind _returnvalue_4 (`GameplayStatics.GetActorOfClass` "/Game/daforma/Blueprints/BP_Transform.BP_Transform_C"))
      (set `/Game/daforma/Blueprints/BP_Transform.RandomEmissiveIntesity` _random_emissive_intesity _returnvalue_4)
      (set `/Game/daforma/Blueprints/BP_Transform.RadiusMask` _radiusmask _returnvalue_4)
      (set `/Game/daforma/Blueprints/BP_Transform.RandomEmissive` _randomemissive _returnvalue_4)
      (set `/Game/daforma/Blueprints/BP_Transform.ModifierEmissive` _modifieremissive _returnvalue_4)
      (set `/Game/daforma/Blueprints/BP_Transform.RandomSeed` _randomseed _returnvalue_4)
      (set `/Game/daforma/Blueprints/BP_Transform.RandomEmissiveTime` _randomemissivetime _returnvalue_4)
      (set `/Game/daforma/Blueprints/BP_Transform.Default Emissive Intesity` _default_emissive_intesity _returnvalue_4)
      (`/Game/daforma/Blueprints/BP_Transform.Start` _returnvalue_4))
    (:`then_4`
      (bind _returnvalue_5 (`GameplayStatics.GetActorOfClass` "/Game/daforma/Blueprints/BP_Ripple.BP_Ripple_C"))
      (set `/Game/daforma/Blueprints/BP_Ripple.RandomEmissiveIntesity` _randomemissivetime _returnvalue_5)
      (set `/Game/daforma/Blueprints/BP_Ripple.RadiusMask` _radiusmask _returnvalue_5)
      (set `/Game/daforma/Blueprints/BP_Ripple.RandomEmissive` _randomemissive _returnvalue_5)
      (set `/Game/daforma/Blueprints/BP_Ripple.ModifierEmissive` _modifieremissive _returnvalue_5)
      (set `/Game/daforma/Blueprints/BP_Ripple.RandomSeed` _randomseed _returnvalue_5)
      (set `/Game/daforma/Blueprints/BP_Ripple.RandomEmissiveTime` _randomemissivetime _returnvalue_5)
      (set `/Game/daforma/Blueprints/BP_Ripple.DefaultEmissiveIntesity` _default_emissive_intesity _returnvalue_5)
      (`/Game/daforma/Blueprints/BP_Ripple.Start` _returnvalue_5))))

(fn `UserConstructionScript`
  (`self.setparameter`))