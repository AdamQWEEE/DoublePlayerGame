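; BP_Jitter is a placeable modifier that drives a material jitter effect, with emissive controls, through the MPC_WPO parameter collection.
; Start writes its location, radius, direction, motion and emissive settings to the collection, resizes the Sphere to match, and overrides Hardness at small radii.
; Start runs on construction and on a looping timer from BeginPlay.
; Construction also calls Setparameter on the BP_Controller found in the level.
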(event `Initialize`
  (bind _returnvalue (`GameplayStatics.GetActorOfClass` "/Game/daforma/Blueprints/BP_Controller.BP_Controller_C"))
  (`/Game/daforma/Blueprints/BP_Controller.setparameter` _returnvalue))

(event `self.ReceiveBeginPlay`
  (`KismetSystemLibrary.K2_SetTimerDelegate` (delegate `Start`) 0.35 true))

(event `Start`
  (bind _radius (`self.Radius`))
  (`|ExecutionSequence`
    (:`then_0`
      (`KismetMaterialLibrary.SetScalarParameterValue` "/Game/daforma/Materials/MPC_WPO.MPC_WPO" "JitterRadius" (`self.Radius`))
      (bind _returnvalue (`KismetMaterialLibrary.GetScalarParameterValue` "/Game/daforma/Materials/MPC_WPO.MPC_WPO" "JitterRadius"))
      (bind _output_get (set `self.Radius` _returnvalue))
      (`SphereComponent.SetSphereRadius` (`self.Sphere`) _output_get true)
      (`KismetMaterialLibrary.SetVectorParameterValue` "/Game/daforma/Materials/MPC_WPO.MPC_WPO" "JitterPosition" (`KismetMathLibrary.Conv_VectorToLinearColor` (`self.K2_GetActorLocation`)))
      (`KismetMaterialLibrary.SetScalarParameterValue` "/Game/daforma/Materials/MPC_WPO.MPC_WPO" "AffectRadius" (`KismetMathLibrary.Conv_BoolToDouble` (`self.RadiusMask`)))
      (`KismetMaterialLibrary.SetScalarParameterValue` "/Game/daforma/Materials/MPC_WPO.MPC_WPO" "RandomEmissive" (`KismetMathLibrary.Conv_BoolToDouble` (`self.RandomEmissive`)))
      (`KismetMaterialLibrary.SetScalarParameterValue` "/Game/daforma/Materials/MPC_WPO.MPC_WPO" "RandomEmissiveTime" (`self.RandomEmissiveTime`))
      (`KismetMaterialLibrary.SetScalarParameterValue` "/Game/daforma/Materials/MPC_WPO.MPC_WPO" "RandomSeed" (`self.RandomSeed`))
      (`KismetMaterialLibrary.SetScalarParameterValue` "/Game/daforma/Materials/MPC_WPO.MPC_WPO" "ModifierEmissive" (`KismetMathLibrary.Conv_BoolToDouble` (`self.ModifierEmissive`)))
      (if (<= _radius 0.0)
        (set `self.Hardness` -100.0)
        (elif (<= _radius 1.0)
          (set `self.Hardness` 0.0)
          (else
            (set `self.Hardness` (`self.Hardness`))))))
    (:`then_1`
      (`KismetMaterialLibrary.SetScalarParameterValue` "/Game/daforma/Materials/MPC_WPO.MPC_WPO" "JitterHardness" (`self.Hardness`))
      (`KismetMaterialLibrary.SetScalarParameterValue` "/Game/daforma/Materials/MPC_WPO.MPC_WPO" "JitterIntensity" (`self.JitterIntensity`)))
    (:`then_2`
      (`KismetMaterialLibrary.SetScalarParameterValue` "/Game/daforma/Materials/MPC_WPO.MPC_WPO" "JitterTime" (`self.JitterTime`))
      (`KismetMaterialLibrary.SetScalarParameterValue` "/Game/daforma/Materials/MPC_WPO.MPC_WPO" "JitterIdleAnim" (`KismetMathLibrary.Conv_BoolToDouble` (`self.JitterIdleAnimation`)))
      (`KismetMaterialLibrary.SetScalarParameterValue` "/Game/daforma/Materials/MPC_WPO.MPC_WPO" "JitterOffset" (`self.JitterOffset`))
      (`KismetMaterialLibrary.SetScalarParameterValue` "/Game/daforma/Materials/MPC_WPO.MPC_WPO" "JitterEmissiveTweakPower" (`self.ModifierEmissiveTweak`))
      (`KismetMaterialLibrary.SetScalarParameterValue` "/Game/daforma/Materials/MPC_WPO.MPC_WPO" "RandomEmissiveIntesity" (`self.Random Emissive Intesity`))
      (`KismetMaterialLibrary.SetScalarParameterValue` "/Game/daforma/Materials/MPC_WPO.MPC_WPO" "DefaultEmissiveIntesity" (`self.DefaultEmissiveIntesity`)))
    (:`then_3`
      (`KismetMaterialLibrary.SetScalarParameterValue` "/Game/daforma/Materials/MPC_WPO.MPC_WPO" "JitterFreq" (`self.JitterFreq`))
      (`KismetMaterialLibrary.SetScalarParameterValue` "/Game/daforma/Materials/MPC_WPO.MPC_WPO" "RandomSeed" (`self.RandomSeed`)))
    (:`then_4`
      (`KismetMaterialLibrary.SetVectorParameterValue` "/Game/daforma/Materials/MPC_WPO.MPC_WPO" "JitterDirection" (`self.JitterDirection`)))))

(fn `UserConstructionScript`
  (`self.Start`)
  (`self.Initialize`))