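; Ripple actor that drives a world position offset and emissive ripple effect in materials through the MPC_WPO parameter collection.
; Start publishes the actor's transform, radius, hardness, direction, animation and emissive settings, resizes its Sphere to the radius and overrides hardness at very small radii.
; Start runs on construction and on a looping timer from BeginPlay instead of Tick.
; Construction also calls Initialize, which triggers Setparameter on BP_Controller.
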(event `Initialize`
  (bind _returnvalue (`GameplayStatics.GetActorOfClass` "/Game/daforma/Blueprints/BP_Controller.BP_Controller_C"))
  (`/Game/daforma/Blueprints/BP_Controller.setparameter` _returnvalue))

(event `self.ReceiveBeginPlay`
  (`KismetSystemLibrary.K2_SetTimerDelegate` (delegate `Start`) 0.35 true))

(event `Start`
  (bind (_returnvalue_roll _returnvalue_pitch _returnvalue_yaw) (`KismetMathLibrary.BreakRotator` (`self.K2_GetActorRotation`)))
  (bind _radius (`self.Radius`))
  (`|ExecutionSequence`
    (:`then_0`
      (`KismetMaterialLibrary.SetScalarParameterValue` "/Game/daforma/Materials/MPC_WPO.MPC_WPO" "RippleSphereRadius" (`self.Radius`))
      (bind _returnvalue (`KismetMaterialLibrary.GetScalarParameterValue` "/Game/daforma/Materials/MPC_WPO.MPC_WPO" "RippleSphereRadius"))
      (bind _output_get (set `self.Radius` _returnvalue))
      (`SphereComponent.SetSphereRadius` (`self.Sphere`) _output_get true)
      (`KismetMaterialLibrary.SetVectorParameterValue` "/Game/daforma/Materials/MPC_WPO.MPC_WPO" "RipplePosition" (`KismetMathLibrary.Conv_VectorToLinearColor` (`self.K2_GetActorLocation`)))
      (`KismetMaterialLibrary.SetVectorParameterValue` "/Game/daforma/Materials/MPC_WPO.MPC_WPO" "RippleRotation" (make `LinearColor` _returnvalue_roll _returnvalue_pitch _returnvalue_yaw 1.0))
      (if (<= _radius 0.0)
        (set `self.Hardness` -100.0)
        (elif (<= _radius 1.0)
          (set `self.Hardness` 0.0)
          (else
            (set `self.Hardness` (`self.Hardness`))))))
    (:`then_1`
      (`KismetMaterialLibrary.SetScalarParameterValue` "/Game/daforma/Materials/MPC_WPO.MPC_WPO" "RippleSphereHardness" (`self.Hardness`)))
    (:`then_2`
      (`KismetMaterialLibrary.SetScalarParameterValue` "/Game/daforma/Materials/MPC_WPO.MPC_WPO" "RippleIntesity" (`self.RippleIntensity`)))
    (:`then_3`
      (`KismetMaterialLibrary.SetVectorParameterValue` "/Game/daforma/Materials/MPC_WPO.MPC_WPO" "RippleDirection" (`self.RippleDirection`)))
    (:`then_4`
      (`KismetMaterialLibrary.SetScalarParameterValue` "/Game/daforma/Materials/MPC_WPO.MPC_WPO" "RippleIdleAnimation" (`KismetMathLibrary.Conv_BoolToDouble` (`self.RippleAnimation`)))
      (`KismetMaterialLibrary.SetScalarParameterValue` "/Game/daforma/Materials/MPC_WPO.MPC_WPO" "RippleFreq" (`self.RippleFreq`))
      (`KismetMaterialLibrary.SetScalarParameterValue` "/Game/daforma/Materials/MPC_WPO.MPC_WPO" "RippleAnimationTime" (`self.RippleAnimationTime`))
      (`KismetMaterialLibrary.SetScalarParameterValue` "/Game/daforma/Materials/MPC_WPO.MPC_WPO" "RippleOffset" (`self.RippleOffset`))
      (`KismetMaterialLibrary.SetScalarParameterValue` "/Game/daforma/Materials/MPC_WPO.MPC_WPO" "DefaultEmissiveIntesity" (`self.DefaultEmissiveIntesity`)))
    (:`then_5`
      (`KismetMaterialLibrary.SetScalarParameterValue` "/Game/daforma/Materials/MPC_WPO.MPC_WPO" "RandomEmissiveTime" (`self.RandomEmissiveTime`))
      (`KismetMaterialLibrary.SetScalarParameterValue` "/Game/daforma/Materials/MPC_WPO.MPC_WPO" "RandomSeed" (`self.RandomSeed`))
      (`KismetMaterialLibrary.SetScalarParameterValue` "/Game/daforma/Materials/MPC_WPO.MPC_WPO" "RandomEmissiveIntesity" (`self.RandomEmissiveIntesity`))
      (`KismetMaterialLibrary.SetScalarParameterValue` "/Game/daforma/Materials/MPC_WPO.MPC_WPO" "AffectRadius" (`KismetMathLibrary.Conv_BoolToDouble` (`self.RadiusMask`)))
      (`KismetMaterialLibrary.SetScalarParameterValue` "/Game/daforma/Materials/MPC_WPO.MPC_WPO" "RandomEmissive" (`KismetMathLibrary.Conv_BoolToDouble` (`self.RandomEmissive`)))
      (`KismetMaterialLibrary.SetScalarParameterValue` "/Game/daforma/Materials/MPC_WPO.MPC_WPO" "RandomEmissiveTime" (`self.RandomEmissiveTime`))
      (`KismetMaterialLibrary.SetScalarParameterValue` "/Game/daforma/Materials/MPC_WPO.MPC_WPO" "RandomSeed" (`self.RandomSeed`))
      (`KismetMaterialLibrary.SetScalarParameterValue` "/Game/daforma/Materials/MPC_WPO.MPC_WPO" "ModifierEmissive" (`KismetMathLibrary.Conv_BoolToDouble` (`self.ModifierEmissive`)))
      (`KismetMaterialLibrary.SetScalarParameterValue` "/Game/daforma/Materials/MPC_WPO.MPC_WPO" "RippleEmissiveTweakPower" (`self.ModifierEmissiveTweak`)))))

(fn `UserConstructionScript`
  (`self.Start`)
  (`self.Initialize`))