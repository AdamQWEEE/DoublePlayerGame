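; BP_Pawn_WalkMesh is a pawn with a skeletal mesh, apparently the walking mannequin used with the InfinityTiles tile spawning.
; At BeginPlay it optionally plays the BP_CamShake camera shake on the first player's camera manager at a configurable scale.
; Its construction script toggles the mesh's first material between a green Matrix text-flow material and the standard mannequin body material.
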(event `self.ReceiveBeginPlay`
  (if (`self.EnableCameraShake?`)
    (`PlayerCameraManager.PlayCameraShake` :`self` (`GameplayStatics.GetPlayerCameraManager` 0) :`ShakeClass` "/Game/InfinityTiles/Blueprints/SpawnTiles/SupportingBP/BP_CamShake.BP_CamShake_C" :`Scale` (`self.CameraShakeScale`))))

(fn `UserConstructionScript`
  (bind _skeletalmesh (`self.SkeletalMesh`))
  (if (`self.UseTextFlowMaterial`)
    (`PrimitiveComponent.SetMaterial` _skeletalmesh 0 "/Game/InfinityTiles/SupportingContent/Mannequin/Character/Materials/MI_MatrixGreen.MI_MatrixGreen")
    (else
      (`PrimitiveComponent.SetMaterial` _skeletalmesh 0 "/Game/InfinityTiles/SupportingContent/Mannequin/Character/Materials/M_UE4Man_Body.M_UE4Man_Body"))))