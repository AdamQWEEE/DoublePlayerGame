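; BP_SpawnTileP is a spawnable tile actor that keeps itself moving continuously in one direction.
; Each Tick it interpolates its root toward a target re-placed at a fixed Offset from its current location, with sweep enabled, so it never arrives.
; The Spawn Manager supplies the direction and speed; ReverseDirection flips the offset, and the interp speed is clamped above zero to avoid a bullet-like jump.
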(event `self.ReceiveTick`
  (params (DeltaSeconds :type "Float (single-precision)"))
  (bind _returnvalue (`self.K2_GetActorLocation`))
  ;[1 1 1] Event Tick
  (`SceneComponent.K2_SetWorldLocation` (`self.DefaultSceneRoot`) (`KismetMathLibrary.VInterpTo` _returnvalue (+ _returnvalue (* (`self.Offset`) (`KismetMathLibrary.SelectInt` -1 1 (`self.ReverseDirection`)))) DeltaSeconds (`KismetMathLibrary.FClamp` (`self.InterpSpeed`) 0.0001)) true false))

(fn `UserConstructionScript`)