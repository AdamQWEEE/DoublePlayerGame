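; Spawn manager for an endless strip of tiles moving along the X axis, with configurable type, scale, speed and direction.
; BeginPlay places two kill-tile actors to destroy tiles and sets visibility of optional level lights.
; It seeds tiles both ways from its root, chaining each at a scaled offset from the previous tile's Sphere marker.
; A self-calling delayed event then keeps appending tiles, with offset compensation against overlap at high speed.
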(event `self.ReceiveBeginPlay`
  ;[0 1 0] [BEGIN PLAY]
  (`self.KillTileSetup`)
  (`self.SpawnSetup`)
  (`self.UseLevelLights`))

(event `KillTileSetup`
  (bind _returnvalue (+ (`SceneComponent.K2_GetComponentLocation` (`self.DefaultSceneRoot`)) (`KismetMathLibrary.MakeVector` (`self.KillTileRange`))))
  ;[1 1 1] Spawn Kill Tile Actor
  (`|SpawnActorFromClass` "/Game/InfinityTiles/Blueprints/SpawnTiles/SupportingBP/BP_KillTile.BP_KillTile_C" (`KismetMathLibrary.MakeTransform` _returnvalue) "AdjustIfPossibleButAlwaysSpawn" "OverrideRootScale" null null) ; Spawns an actor that destroys the tiles
  (`|SpawnActorFromClass` "/Game/InfinityTiles/Blueprints/SpawnTiles/SupportingBP/BP_KillTile.BP_KillTile_C" (`KismetMathLibrary.MakeTransform` (* _returnvalue -1.0)) "AdjustIfPossibleButAlwaysSpawn" "OverrideRootScale" null null) ; Spawns an actor that destroys the tiles
)

(event `SpawnSetup`
  (bind _uniformtilescale (`self.UniformTileScale`))
  ;[1 1 1] Initial Tile Set Spawn Configuration
  (set `self.TileScale` (`KismetMathLibrary.MakeVector` _uniformtilescale _uniformtilescale _uniformtilescale))
  (set `self.TileOffset` (* (1500.0 0.0 0.0) _uniformtilescale))
  (`self.InitialSpawn`)
  (set `self.Direction` (`KismetMathLibrary.SelectInt` 1 -1 (`self.ReverseTileDirection`))) ; Spawn in both sides around the center of this actor
  (set `self.LastTile` (`self.FirstTile`))
  (`self.InitialSpawn`)
  (`self.ContinuousSpawn`))

(event `InitialSpawn`
  (bind _reversetiledirection (`self.ReverseTileDirection`))
  (bind _spawntiletype (`self.SpawnTileType`))
  (bind _lasttile (`self.LastTile`))
  (bind _returnvalue (`KismetMathLibrary.MakeTransform` (`self.SpawnLocation`) (struct) (`self.TileScale`)))
  (bind _returnvalue_2 (`KismetMathLibrary.FClamp` (`self.TileSpeed`)))
  ;[1 1 1] Initial Tile Set Spawn
  (for _ (range (+ (`self.InitialTilesAmount`) 1))
    (`/Engine/EditorBlueprintResources/StandardMacros.IsValid` _lasttile
      (:`Is Valid`
        (set `self.SpawnLocation` (+ (`SceneComponent.K2_GetComponentLocation` (`/Game/InfinityTiles/Blueprints/SpawnTiles/SupportingBP/BP_SpawnTileP.Sphere` _lasttile)) (* (`self.TileOffset`) (`self.Direction`)))) ; Spawn a new tile at a location that is at a constant offset \n(i.e. the size of tile) from the previously spawned tile
        (bind _returnvalue_3 (`|SpawnActorFromClass` _spawntiletype _returnvalue "Undefined" "OverrideRootScale" null _returnvalue_2 _reversetiledirection null))
        (set `self.LastTile` _returnvalue_3) ; Set a reference to the last tile spawned by this actor\nfor location info
      )
      (:`Is Not Valid`
        (set `self.SpawnLocation` (`SceneComponent.K2_GetComponentLocation` (`self.DefaultSceneRoot`))) ; Spawn at root if it is the first time we are spawnning a tile
        (bind _returnvalue_4 (`|SpawnActorFromClass` _spawntiletype _returnvalue "Undefined" "OverrideRootScale" null _returnvalue_2 _reversetiledirection null))
        (bind _output_get (set `self.FirstTile` _returnvalue_4)) ; This is used to prevent\noverlap case of first run
        (set `self.LastTile` _output_get) ; Set a reference to the last tile spawned by this actor\nfor location info
      ))))

(event `ContinuousSpawn`
  (bind _direction (`self.Direction`))
  (bind _lasttile (`self.LastTile`))
  ;[1 1 1] Continuous Tile Spawn
  (`KismetSystemLibrary.Delay` (`self.SpawnDelay`))
  (`/Engine/EditorBlueprintResources/StandardMacros.IsValid` _lasttile
    (:`Is Valid`
      (set `self.SpawnLocation` (+ (`SceneComponent.K2_GetComponentLocation` (`/Game/InfinityTiles/Blueprints/SpawnTiles/SupportingBP/BP_SpawnTileP.Sphere` _lasttile)) (* (`self.TileOffset`) _direction) (* (`KismetMathLibrary.MakeVector` (`self.OffsetCompensation`)) _direction))) ; Spawn a new tile at a location that is at a constant offset \n(i.e. the size of tile) from the previously spawned tile
    )
    (:`Is Not Valid`
      (set `self.SpawnLocation` (`SceneComponent.K2_GetComponentLocation` (`self.DefaultSceneRoot`))) ; This path should never take place, but is here for error evaluation if it occurs
    ))
  (bind _returnvalue (`|SpawnActorFromClass` (`self.SpawnTileType`) (`KismetMathLibrary.MakeTransform` (`self.SpawnLocation`) (struct) (`self.TileScale`)) "Undefined" "OverrideRootScale" null (`KismetMathLibrary.FClamp` (`self.TileSpeed`)) (`self.ReverseTileDirection`) null))
  (set `self.LastTile` _returnvalue)
  (`self.ContinuousSpawn`) ; Call itself event again to spawn the next tile\nThis essentially creates an infinite looping event call\nthat get triggered after a certain delay
)

(event `UseLevelLights`
  (bind _levellight1 (`self.LevelLight1`))
  (bind _levellightshidden (`self.LevelLightsHidden`))
  (bind _levellight2 (`self.LevelLight2`))
  ;[1 1 1] Enable / Disable Level Lights (Set actor reference in level before use)
  (`/Engine/EditorBlueprintResources/StandardMacros.IsValid` _levellight1
    (:`Is Valid`
      (`self.SetActorHiddenInGame` _levellight1 _levellightshidden)
      (`/Engine/EditorBlueprintResources/StandardMacros.IsValid` _levellight2
        (:`Is Valid`
          (`self.SetActorHiddenInGame` _levellight2 _levellightshidden))))))

(fn `UserConstructionScript`
  (set `self.Direction` (`KismetMathLibrary.SelectInt` -1 1 (`self.ReverseTileDirection`))) ; Set the initial value based on "Reverse Direction"
)