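; BP_HexSpin is a procedural tile actor that builds a spinning, spiral-twisted row of hexagon meshes.
; The Construction Script computes a scale-adjusted X offset, then SpawnX adds static mesh components along that axis with the exposed material and non-uniform scale.
; An accumulated roll offset creates the twist between meshes, while a RotatingMovement component rolls the whole actor at a configurable speed.
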(event `SpawnX`
  (params (MaxCount :type Integer))
  (bind _nexttransformsx_location (`KismetMathLibrary.BreakTransform` (`self.NextTransformsX`)))
  (bind _nextrotationoffset (`self.NextRotationOffset`))
  ;[1 1 1] Spawn Mesh in X direction
  (for _ (range (+ MaxCount 1))
    (bind _returnvalue (`AddComponent|NODE_AddStaticMeshComponent-2` :`RelativeTransform` (`self.NextTransformsX`))) ; Add a Hexagon Static Mesh
    (`PrimitiveComponent.SetMaterial` _returnvalue 0 (`self.HexagonMaterial1`)) ; Sets the material of the mesh\nfrom the variable exposed to \nTile BP
    (set `self.NextTransformsX` (`KismetMathLibrary.MakeTransform` (+ _nexttransformsx_location (`self.XOffset`)) _nextrotationoffset (`KismetMathLibrary.MakeVector` (`self.ScaleX`) (`self.ScaleY`) (`self.ScaleZ`)))) ; Sets the next spawn transforms
    (set `self.NextRotationOffset` (`KismetMathLibrary.ComposeRotators` _nextrotationoffset (`KismetMathLibrary.MakeRotator` (`self.RotationOffset`)))) ; This is the result of Last Mesh Rotation combined with Rotation Offset
  ))

(fn `UserConstructionScript`
  (bind _scalex (`self.ScaleX`))
  (set `self.XOffset` (`KismetMathLibrary.MakeVector` (* (`self.OffsetDistance`) _scalex))) ; This is the X direction scaled offset
  (set `self.NextTransformsX` (`KismetMathLibrary.MakeTransform` (0.0 0.0 0.0) (`self.NextRotationOffset`) (`KismetMathLibrary.MakeVector` _scalex (`self.ScaleY`) (`self.ScaleZ`))))
  (`self.SpawnX` (`self.X_Count`))
  (set `RotatingMovementComponent.RotationRate` (`KismetMathLibrary.MakeRotator` (`self.RotationSpeed`)) (`self.RotatingMovement`)))