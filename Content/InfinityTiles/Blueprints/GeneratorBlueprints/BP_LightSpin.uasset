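; BP_LightSpin is a generator actor that builds a spinning ring of BP_LightPanel actors around its forward axis.
; The Construction Script sets the RotatingMovement roll rate, then calls SpawnPanel to add evenly spaced child actor components at a configurable count, spread and scale.
; Each panel receives the shared material and attaches to the root, so it turns with the ring as well as on its own axis.
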(event `SpawnPanel`
  (bind _returnvalue (`self.GetActorForwardVector`))
  (bind _angle (`self.Angle`))
  (bind _count (`self.Count`))
  (bind _uniformscale (`self.UniformScale`))
  (bind _returnvalue_2 (`KismetMathLibrary.MakeTransform` (+ (`self.K2_GetActorLocation`) (`KismetMathLibrary.RotateAngleAxis` (* (`self.GetActorUpVector`) (`self.Spread`)) _angle _returnvalue)) (`KismetMathLibrary.RotatorFromAxisAndAngle` _returnvalue _angle) (`KismetMathLibrary.MakeVector` _uniformscale _uniformscale _uniformscale)))
  ;[1 1 1] Spawn Light Panels
  (set `self.NextTransforms` _returnvalue_2)
  (set `self.AngelIncrement` (/ 360.0 (`KismetMathLibrary.Conv_IntToDouble` _count))) ; This is changed depending on the\nnumber of Panels we wan to spawn\n(360 divided by Number of Panels)
  (for _ (range 1 (+ _count 1))
    (bind _returnvalue_3 (`AddComponent|NODE_AddChildActorComponent-0` :`bManualAttachment` true :`RelativeTransform` (`self.NextTransforms`)))
    (bind _asbp_light_panel (cast `/Game/InfinityTiles/Blueprints/GeneratorBlueprints/BP_LightPanel` (`ChildActorComponent.ChildActor` _returnvalue_3)))
    (set `/Game/InfinityTiles/Blueprints/GeneratorBlueprints/BP_LightPanel.PanelMaterial` (`self.PanelMaterial`) _asbp_light_panel) ; Set the material of Light Panel
    (`SceneComponent.K2_AttachToComponent` _returnvalue_3 (`self.DefaultSceneRoot`) "None" "KeepWorld" "KeepRelative" "KeepRelative" true) ; Set the attachment so it rotates on its own axis \nas well as this actor axis
    (set `self.Angle` (+ (`self.Angle`) (`self.AngelIncrement`))) ; Angle of the next Panel
    (set `self.NextTransforms` _returnvalue_2) ; Transforms of the next panel
  ))

(fn `UserConstructionScript`
  (set `RotatingMovementComponent.RotationRate` (`KismetMathLibrary.MakeRotator` (`self.RotationRate`)) (`self.RotatingMovement`))
  (`self.SpawnPanel`) ; Spawn Rotating Light Panels
)