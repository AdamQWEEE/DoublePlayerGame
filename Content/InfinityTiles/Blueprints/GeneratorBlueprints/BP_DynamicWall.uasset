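; Procedural wall generator that builds a grid of cube static mesh components in the construction script.
; The construction script derives step offsets from the uniform cube scale, then SpawnXY stacks ZCount rows, calling SpawnX to lay XCount cubes along each.
; Each cube gets the configured material and a random Y depth offset within RandomVariance, kept out of the running transforms so the grid spacing stays even.
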(event `SpawnX`
  (params (MaxCount :type Integer))
  (bind _nexttransformsx_location (`KismetMathLibrary.BreakTransform` (`self.NextTransformsX`)))
  (bind (_nexttransformsx_location_2 _nexttransformsx_rotation _nexttransformsx_scale) (`KismetMathLibrary.BreakTransform` (`self.NextTransformsX`)))
  (bind _uniformscale (`self.UniformScale`))
  (bind _randomvariance (`self.RandomVariance`))
  ;[1 1 1] Spawn in the X direction
  (for _ (range (+ MaxCount 1))
    (bind _returnvalue (`AddComponent|NODE_AddStaticMeshComponent-2` :`RelativeTransform` (`KismetMathLibrary.MakeTransform` (+ _nexttransformsx_location_2 (`KismetMathLibrary.MakeVector` 0.0 (`KismetMathLibrary.RandomFloatInRange` (* _randomvariance -1.0) _randomvariance))) _nexttransformsx_rotation _nexttransformsx_scale))) ; Adds a Cube Static Mesh dynamically
    (`PrimitiveComponent.SetMaterial` _returnvalue 0 (`self.CubeMaterial`)) ; Set the material of the cube mesh
    (set `self.NextTransformsX` (`KismetMathLibrary.MakeTransform` (+ _nexttransformsx_location (`self.XOffset`)) (struct) (`KismetMathLibrary.MakeVector` _uniformscale _uniformscale _uniformscale))) ; Use this transform for the next cube\nThis does not contain the depth randomness\nand has the constant offset for next cube which\nis equal to the size of the cube
  ))

(event `SpawnXY`
  (params (MaxCount :type Integer))
  (bind _uniformscale (`self.UniformScale`))
  (bind _nexttransformsz_location (`KismetMathLibrary.BreakTransform` (`self.NextTransformsZ`)))
  (bind _returnvalue (`KismetMathLibrary.MakeVector` _uniformscale _uniformscale _uniformscale))
  (bind _returnvalue_2 (+ _nexttransformsz_location (`self.ZOffset`)))
  ;[1 1 1] Set Spawn Location in the Z direction
  (for _ (range (+ MaxCount 1))
    (`self.SpawnX` (`self.X_Count`))
    (set `self.NextTransformsX` (`KismetMathLibrary.MakeTransform` _returnvalue_2 (struct) _returnvalue)) ; Move one step upwards for Spawn X
    (set `self.NextTransformsZ` (`KismetMathLibrary.MakeTransform` _returnvalue_2 (struct) _returnvalue)) ; Set the next "Up" step value
  ))

(fn `UserConstructionScript`
  (bind _uniformscale (`self.UniformScale`))
  (bind _returnvalue (`KismetMathLibrary.MakeVector` _uniformscale _uniformscale _uniformscale))
  (set `self.XOffset` (`KismetMathLibrary.MakeVector` (* 20.0 _uniformscale))) ; Offset used to place the next cube in X
  (set `self.ZOffset` (`KismetMathLibrary.MakeVector` 0.0 0.0 (* 20.0 _uniformscale))) ; Offset used to place the next cube in Z
  (set `self.NextTransformsX` (`KismetMathLibrary.MakeTransform` (10.0 0.0 0.0) (struct) _returnvalue)) ; Set initial values of the X direction transform
  (set `self.NextTransformsZ` (`KismetMathLibrary.MakeTransform` (10.0 0.0 0.0) (struct) _returnvalue)) ; Set initial values of the Z direction transform
  (`self.SpawnXY` (`self.Z_Count`)))