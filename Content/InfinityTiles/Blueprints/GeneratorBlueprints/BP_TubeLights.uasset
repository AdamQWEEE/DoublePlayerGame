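; BP_TubeLights is a generator Blueprint that builds a row of tube static meshes along X at construction time.
; The construction script derives a scaled spacing and first transform, lifting tubes so their base meets the Blueprint origin, then calls SpawnX.
; SpawnX adds each mesh component with random Y depth variance, sizing length separately from uniform scale.
; An optional FlipFlop alternates two materials between successive tubes.
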(event `SpawnX`
  (params (MaxCount :type Integer))
  (bind _nexttransformsx_location (`KismetMathLibrary.BreakTransform` (`self.NextTransformsX`)))
  (bind (_nexttransformsx_location_2 _nexttransformsx_rotation _nexttransformsx_scale) (`KismetMathLibrary.BreakTransform` (`self.NextTransformsX`)))
  (bind _uniformscale (`self.UniformScale`))
  (bind _randomvariance (`self.RandomVariance`))
  (for _ (range (+ MaxCount 1))
    (bind _returnvalue (`AddComponent|NODE_AddStaticMeshComponent-2` :`RelativeTransform` (`KismetMathLibrary.MakeTransform` (+ _nexttransformsx_location_2 (`KismetMathLibrary.MakeVector` 0.0 (`KismetMathLibrary.RandomFloatInRange` (* _randomvariance -1.0) _randomvariance))) _nexttransformsx_rotation _nexttransformsx_scale))) ; Add the Tube Static Mesh
    (if (`self.AlternateMaterials`)
      (`/Engine/EditorBlueprintResources/StandardMacros.FlipFlop`
        (:`A`
          (`PrimitiveComponent.SetMaterial` _returnvalue 0 (`self.TubeMaterial1`)))
        (:`B`
          (`PrimitiveComponent.SetMaterial` _returnvalue 0 (`self.TubeMaterial2`))))
      (else
        (`PrimitiveComponent.SetMaterial` _returnvalue 0 (`self.TubeMaterial1`))))
    (set `self.NextTransformsX` (`KismetMathLibrary.MakeTransform` (+ _nexttransformsx_location (`self.XOffset`)) (struct :`Pitch` 90.0) (`KismetMathLibrary.MakeVector` (+ (`self.LengthScale`) _uniformscale) _uniformscale _uniformscale)))))

(fn `UserConstructionScript`
  (bind _uniformscale (`self.UniformScale`))
  (bind _returnvalue (+ _uniformscale (`self.LengthScale`)))
  (set `self.XOffset` (`KismetMathLibrary.MakeVector` (* (`self.OffsetDistance`) _uniformscale))) ; Scaled offset for next Tube location
  (set `self.NextTransformsX` (`KismetMathLibrary.MakeTransform` (`KismetMathLibrary.MakeVector` 0.0 0.0 (* _returnvalue 100.0)) (struct :`Pitch` 90.0) (`KismetMathLibrary.MakeVector` _returnvalue _uniformscale _uniformscale)))
  (`self.SpawnX` (`self.X_Count`)))