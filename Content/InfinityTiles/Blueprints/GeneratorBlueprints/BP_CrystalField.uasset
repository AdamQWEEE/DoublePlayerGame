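; BP_CrystalField is a generator Blueprint that procedurally scatters crystals and optional rubble patches within a configurable box area.
; Its construction script calls spawn events by configurable counts, each adding a static mesh component at a random point in the box.
; Crystals get a random mesh, random roll and pitch, and uniform scale.
; Rubble stays unrotated, scales only horizontally, and gets a dynamic material instance from a randomly picked material.
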(event `SpawnCrystal`
  (bind _crystalstype (`self.CrystalsType`))
  (bind _crystalsize (`self.CrystalSize`))
  (bind _crystalrollrange (`self.CrystalRollRange`))
  (bind _crystalpitchrange (`self.CrystalPitchRange`))
  ;[1 1 1] Spawn Crystals
  (bind _returnvalue (`AddComponent|NODE_AddStaticMeshComponent-0` :`RelativeTransform` (`KismetMathLibrary.MakeTransform` (`KismetMathLibrary.RandomPointInBoundingBox` (0.0 0.0 0.0) (`KismetMathLibrary.MakeVector` (`self.BoxSizeX`) (`self.BoxSizeY`) 1.0)) (`KismetMathLibrary.MakeRotator` (`KismetMathLibrary.RandomFloatInRange` (* -1 _crystalrollrange) _crystalrollrange) (`KismetMathLibrary.RandomFloatInRange` (* -1 _crystalpitchrange) _crystalpitchrange)) (`KismetMathLibrary.MakeVector` _crystalsize _crystalsize _crystalsize)))) ; Add an empty Static Mesh Component dynamically
  (`StaticMeshComponent.SetStaticMesh` _returnvalue (`|GetArrayItem` _crystalstype (`KismetMathLibrary.RandomIntegerInRange` 0 (- (`KismetArrayLibrary.Array_Length` _crystalstype) 1)))) ; Set it to a random crystal mesh
)

(event `SpawnRubble`
  (bind _rubblematerialtypes (`self.RubbleMaterialTypes`))
  (bind _rubblescale (`self.RubbleScale`))
  ;[1 1 1] Spawn Rubble
  (bind _returnvalue (`AddComponent|NODE_AddStaticMeshComponent-1` :`RelativeTransform` (`KismetMathLibrary.MakeTransform` (`KismetMathLibrary.RandomPointInBoundingBox` (0.0 0.0 0.0) (`KismetMathLibrary.MakeVector` (`self.BoxSizeX`) (`self.BoxSizeY`) 1.0)) (struct) (`KismetMathLibrary.MakeVector` _rubblescale _rubblescale 1.0)))) ; Add a Static Mesh Component and set it to Rubble dynamically
  (`PrimitiveComponent.CreateDynamicMaterialInstance` _returnvalue 0 (`|GetArrayItem` _rubblematerialtypes (`KismetMathLibrary.RandomIntegerInRange` 0 (- (`KismetArrayLibrary.Array_Length` _rubblematerialtypes) 1))) "None") ; Randomize the material of the rubble
)

(fn `UserConstructionScript`
  (for _ (range (+ (`self.CrystalCount`) 1))
    (`self.SpawnCrystal`) ; Spawns Crystals, amount is specified by Crystal Count
  )
  (if (`self.SpawnRubble?`)
    (for _ (range (+ (`self.RubblePatchCount`) 1))
      (`self.SpawnRubble`) ; Checks if we can spawn rubble first\nSpawns Rubble, amount is specified by Rubble Patch Count
    )))