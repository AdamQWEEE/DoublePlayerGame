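; BP_ShowcaseFull is a showcase prop with a base, glass and two rect lights, all tinted by one shared color.
; The construction script creates dynamic material instances for the Base and Glass meshes and sets their EmissiveColor parameter to CommonColor.
; It applies the same CommonColor, exposed for calling Blueprints, to the upper and lower rect lights.
; The event graph holds no active logic.
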(fn `UserConstructionScript`
  (bind _commoncolor (`self.CommonColor`))
  ;[1 1 1] Set the same color for each component
  (bind _returnvalue (`PrimitiveComponent.CreateDynamicMaterialInstance` (`self.Base`) 0 "/Game/InfinityTiles/Materials/ShowcaseBox/MI_Showcase_Base_T1.MI_Showcase_Base_T1" "None"))
  (`MaterialInstanceDynamic.SetVectorParameterValue` _returnvalue "EmissiveColor" _commoncolor)
  (bind _returnvalue_2 (`PrimitiveComponent.CreateDynamicMaterialInstance` (`self.Glass`) 0 "/Game/InfinityTiles/Materials/ShowcaseBox/MI_Showcase_Glass_T1.MI_Showcase_Glass_T1" "None"))
  (`MaterialInstanceDynamic.SetVectorParameterValue` _returnvalue_2 "EmissiveColor" _commoncolor)
  (`LightComponent.SetLightColor` (`self.RectLightUP`) _commoncolor true)
  (`LightComponent.SetLightColor` (`self.RectLightDN`) _commoncolor true))